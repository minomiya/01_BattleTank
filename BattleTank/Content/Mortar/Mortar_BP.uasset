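; Mortar actor with a turret, a barrel and a health bar widget.
; On BeginPlay it passes the MortarTurret and MortarBarrel components to its TankAiming component for aiming setup.
; It then casts the Widget component's user widget to HealthBar and sets that widget's MyTank reference to itself, linking the bar to this mortar.
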(event EventBeginPlay
  (Class|TankAimingComponent|Initialise (Variables|Default|GetTankAiming) (Variables|Default|GetMortarTurret) (Variables|Default|GetMortarBarrel))
  (CallFunction|InitialiseHealthBar))

(fn ConstructionScript)

(fn InitialiseHealthBar
  (bind _ashealth_bar (Utilities|Casting|CastToHealthBar (UserInterface|GetUserWidgetObject (Variables|Default|GetWidget))))
  (Variables|/Game/UI/HealthBar.HealthBar_C|SetMyTank _ashealth_bar self))